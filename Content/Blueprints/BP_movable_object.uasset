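; BP_movable_object is a throwable physics actor that copies the mesh of another movable object it hits while thrown.
; Throw sets the Thrown flag, which Tick clears once the mesh's physics velocity reaches zero.
; On Hit, a thrown object takes the static mesh of the other BP_movable_object.
; ChangeTexture turns the mesh red and spawns a duplicate with the same mesh at a random location above zero height.
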(event `self.ReceiveTick`
  (params (DeltaSeconds :type "Float (single-precision)"))
  (if (`self.Thrown`)
    (bind _returnvalue (`PrimitiveComponent.GetPhysicsLinearVelocity` (`self.StaticMesh`) "None"))
    (if (== _returnvalue (0.0 0.0 0.0))
      (set `self.Thrown` false))))

(event `self.ReceiveHit`
  (params (MyComp :type "PrimitiveComponent Object Reference") (Other :type "Actor Object Reference") (OtherComp :type "PrimitiveComponent Object Reference") (bSelfMoved :type Boolean) (HitLocation :type "Vector Structure") (HitNormal :type "Vector Structure") (NormalImpulse :type "Vector Structure") (Hit :type "HitResult Structure (by ref)"))
  (if (and (`self.Thrown`) (`KismetSystemLibrary.IsValid` Other))
    (if (== (`GameplayStatics.GetObjectClass` Other) "BP_movable_object_C")
      (bind _asbp_movable_object (cast `/Game/Blueprints/BP_movable_object` Other))
      (`StaticMeshComponent.SetStaticMesh` (`self.StaticMesh`) (`StaticMeshComponent.StaticMesh` (`/Game/Blueprints/BP_movable_object.StaticMesh` _asbp_movable_object))) ; Set this static mesh to the one of the hit object
    )))

(fn `ChangeTexture`
  (`PrimitiveComponent.SetMaterial` (`self.StaticMesh`) 0 "/Game/Materials/M_Red.M_Red")
  (bind _returnvalue (`|SpawnActorFromClass` "BP_movable_object_C" (`KismetMathLibrary.MakeTransform` (`KismetMathLibrary.MakeVector` (.x (* (`KismetMathLibrary.RandomUnitVector`) 2000)) (.y (* (`KismetMathLibrary.RandomUnitVector`) 2000)) (`KismetMathLibrary.Abs` (.z (* (`KismetMathLibrary.RandomUnitVector`) 2000))))) "Undefined" "MultiplyWithRoot" null null))
  (`StaticMeshComponent.SetStaticMesh` (`/Game/Blueprints/BP_movable_object.StaticMesh` _returnvalue) (`StaticMeshComponent.StaticMesh` (`self.StaticMesh`))) ; Give new actor same static mesh as this actor
)

(fn `Throw`
  (set `self.Thrown` true))

(fn `UserConstructionScript`)